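; BP_PlayerCharachter is the player character, with a health component, a widget healthbar and a tintable body.
; On BeginPlay it creates the game HUD and colors the healthbar green or red by its "Friendly" tag.
; BPC_Health events refresh the healthbar percentage on damage or heal, and on death destroy the actor and notify BP_MainGamemode.
; The construction script applies BodyColor through a dynamic material instance on the mesh.
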(event OnDead(BPC_Health)
  (Actor|DestroyActor)
  (bind _asbp_main_gamemode (Utilities|Casting|CastToBP_MainGamemode (Game|GetGameMode)))
  (Default|PlayerDied _asbp_main_gamemode))

(event OnDamage(BPC_Health)
  (bind _asbpw_healthbar (Utilities|Casting|CastToBPW_Healthbar (UserInterface|GetWidget (Variables|Default|GetHealthbar))))
  (Variables|/Game/Blueprints/HUD/BPW_Healthbar.BPW_Healthbar_C|SetCurrentHealthPercentage _asbpw_healthbar (Default|GetHealthPercentage (Variables|Default|GetBPC_Health))))

(event OnHeal(BPC_Health)
  (bind _asbpw_healthbar (Utilities|Casting|CastToBPW_Healthbar (UserInterface|GetWidget (Variables|Default|GetHealthbar))))
  (Variables|/Game/Blueprints/HUD/BPW_Healthbar.BPW_Healthbar_C|SetCurrentHealthPercentage _asbpw_healthbar (Default|GetHealthPercentage (Variables|Default|GetBPC_Health))))

(event EventBeginPlay
  (|CallParentFunction)
  (Utilities|FlowControl|Sequence
    (:then_0
      ;[1 1 1] Setup HUD
      (bind _returnvalue (UserInterface|CreateWidget "/Game/Blueprints/HUD/BPW_GameHUD.BPW_GameHUD_C"))
      (UserInterface|Viewport|AddtoViewport _returnvalue 0))
    (:then_1
      (bind _asbpw_healthbar (Utilities|Casting|CastToBPW_Healthbar (UserInterface|GetWidget (Variables|Default|GetHealthbar))))
      (Variables|/Game/Blueprints/HUD/BPW_Healthbar.BPW_Healthbar_C|SetHealthColor _asbpw_healthbar (Math|Color|SelectColor "(R=0.979167,G=0.020399,B=0.040779,A=1.000000)" "(R=0.036250,G=0.966667,B=0.152849,A=1.000000)" (not (Utilities|Array|ContainsItem (Variables|Actor|GetTags) "Friendly")))))))

(event Collision|EventActorBeginOverlap
  (params (OtherActor :type Actor%20Object%20Reference)))

(event EventTick
  (params (DeltaSeconds :type Float%20%28single-precision%29)))

(fn ConstructionScript
  (bind _returnvalue (Rendering|Material|CreateDynamicMaterialInstance (Variables|Character|GetMesh) 0 0 "None" :!class /Script/Engine.PrimitiveComponent))
  (bind _output_get (Variables|Default|SetMaterialInstance _returnvalue))
  (Rendering|Material|SetVectorParameterValue _output_get "BodyColor" (Variables|Default|GetBodyColor) :!class /Script/Engine.MaterialInstanceDynamic))