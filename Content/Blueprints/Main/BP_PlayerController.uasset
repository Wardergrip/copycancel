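; Player controller for a top-down-style game with cursor aiming, abilities and a minion and upgrade shop.
; It spawns a BP_AbilityManager that receives primary fire, cursor target locations and cast cancels from movement input.
; Mouse movement traces under the cursor to yaw the control rotation toward the hit point.
; Shop keys forward purchases to BP_MainGamemode, and Tick deals lethal damage when the pawn falls below a height limit.
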(event EventBeginPlay
  (bind _returnvalue (Game|SpawnActorfromClass "/Game/Blueprints/BP_AbilityManager.BP_AbilityManager_C" (Math|Transform|MakeTransform "0, 0, 0" "0, 0, 0" "1,1,1") "Undefined" 0 0))
  (Variables|Default|SetAbilityManager _returnvalue))

(event EventTick
  (params (DeltaSeconds :type Float%20%28single-precision%29))
  (bind _returnvalue (Pawn|GetControlledPawn))
  (if (<= (.z (Transformation|GetActorLocation _returnvalue)) -3e+02)
    (Default|DealDamage (Utilities|Array|Get(acopy) (Actor|GetComponentsByClass _returnvalue "/Game/Blueprints/BPC_Health.BPC_Health_C")) 99999.0)))

(event Input|ActionEvents|InputActionPrimaryFire
  (params (Key :type Key%20Structure :default "None"))
  (:Pressed
    (Default|PrimaryFire (Variables|Default|GetAbilityManager))))

(event Input|ActionEvents|InputActionShopBuy1
  (params (Key :type Key%20Structure :default "None"))
  (:Pressed
    (bind _asbp_main_gamemode (Utilities|Casting|CastToBP_MainGamemode (Game|GetGameMode)))
    (Default|TryBuyNewMinion _asbp_main_gamemode)))

(event Input|ActionEvents|InputActionShopBuy2
  (params (Key :type Key%20Structure :default "None"))
  (:Pressed
    (bind _asbp_main_gamemode (Utilities|Casting|CastToBP_MainGamemode (Game|GetGameMode)))
    (Default|TryBuyDamage _asbp_main_gamemode)))

(event Input|ActionEvents|InputActionShopBuy3
  (params (Key :type Key%20Structure :default "None"))
  (:Pressed
    (bind _asbp_main_gamemode (Utilities|Casting|CastToBP_MainGamemode (Game|GetGameMode)))
    (Default|TryBuyHealth _asbp_main_gamemode)))

(event Input|ActionEvents|InputActionShopBuy4
  (params (Key :type Key%20Structure :default "None"))
  (:Pressed
    (bind _asbp_main_gamemode (Utilities|Casting|CastToBP_MainGamemode (Game|GetGameMode)))
    (Default|TryBuyHealingPower _asbp_main_gamemode)))

(event Input|AxisEvents|InputAxisMoveVertical
  (params (AxisValue :type Float%20%28single-precision%29))
  ;[1 1 1] Handle movement input
  (Pawn|Input|AddMovementInput (Pawn|GetControlledPawn) "1.000000, 0, 0" AxisValue false)
  (if (> (Math|Float|Square (+ AxisValue (stale Input|AxisEvents|InputAxisMoveHorizontal AxisValue))) 0.0)
    (Default|CancelAbilityCast (Variables|Default|GetAbilityManager)) ; Movement cancels ability casting
  ))

(event Input|AxisEvents|InputAxisMoveHorizontal
  (params (AxisValue :type Float%20%28single-precision%29))
  ;[1 1 1] Handle movement input
  (Pawn|Input|AddMovementInput (Pawn|GetControlledPawn) "0,1.000000, 0" AxisValue false)
  (if (> (Math|Float|Square (+ (stale Input|AxisEvents|InputAxisMoveVertical AxisValue) AxisValue)) 0.0)
    (Default|CancelAbilityCast (Variables|Default|GetAbilityManager)) ; Movement cancels ability casting
  ))

(event Input|AxisEvents|InputAxisCycleThrough
  (params (AxisValue :type Float%20%28single-precision%29)))

(event Input|MouseEvents|MouseX
  (params (AxisValue :type Float%20%28single-precision%29))
  (bind (_hitresult _returnvalue) (Game|Player|GetHitResultUnderCursorbyChannel "TraceTypeQuery1" true))
  (bind _location (Collision|BreakHitResult _hitresult))
  (if _returnvalue
    (Pawn|SetControlRotation (Math|Rotator|MakeRotator 0.0 0.0 (.yaw (Math|Rotator|FindLookatRotation (Transformation|GetActorLocation (Pawn|GetControlledPawn)) _location))))
    (Default|ChangeLocation (Variables|Default|GetAbilityManager) _location)))

(event Input|MouseEvents|MouseY
  (params (AxisValue :type Float%20%28single-precision%29))
  (bind (_hitresult _returnvalue) (Game|Player|GetHitResultUnderCursorbyChannel "TraceTypeQuery1" true))
  (bind _location (Collision|BreakHitResult _hitresult))
  (if _returnvalue
    (Pawn|SetControlRotation (Math|Rotator|MakeRotator 0.0 0.0 (.yaw (Math|Rotator|FindLookatRotation (Transformation|GetActorLocation (Pawn|GetControlledPawn)) _location))))
    (Default|ChangeLocation (Variables|Default|GetAbilityManager) _location)))

(fn ConstructionScript)