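; Main game mode that tracks coins and score, sells minion upgrades and restarts the level on player death.
; Purchases spawn friendly minions near the player or raise damage, max health or healing power, pushing stats to live actors and increasing each price.
; Tutorial0 grants starting coins, raises the enemy cap on a timer and opens Sandbox once no enemies remain.
; Elsewhere, any minion death scales enemy stats and raises the cap by score.
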(event Custom|PlayerDied
  (bind _returnvalue (Game|GetCurrentLevelName true))
  (Game|OpenLevel(byName) (Utilities|String|StringToName _returnvalue)))

(event Custom|AddCoins
  (params (Amount :type Integer))
  (Variables|Default|SetCoins (+ Amount (Variables|Default|GetCoins)))
  (Variables|Default|SetScore (+ Amount (Variables|Default|GetScore))))

(event Custom|SubstractCoins
  (params (Amount :type Integer))
  (Variables|Default|SetCoins (- (Variables|Default|GetCoins) Amount)))

(event Custom|TryBuyNewMinion
  (bind _returnvalue (Game|Player|GetPlayerPawn 0))
  (bind _returnvalue_2 (Math|Random|RandomUnitVector))
  (if (>= (Variables|Default|GetCoins) (Variables|Default|GetCostNewMinion))
    (CallFunction|SubstractCoins (Variables|Default|GetCostNewMinion))
    (AI|SpawnAIFromClass "/Game/Blueprints/BP_FriendlyMinion.BP_FriendlyMinion_C" 0 (+ (Transformation|GetActorLocation _returnvalue) (* (Math|Vector|MakeVector (.x _returnvalue_2) (.y _returnvalue_2) (Math|Float|Absolute(Float) (.z _returnvalue_2))) 1e+02)) (Transformation|GetActorRotation _returnvalue) false 0)
    (Variables|Default|SetCostNewMinion (+ (Variables|Default|GetCostNewMinion) (/ (Variables|Default|GetCostNewMinion) 4)))))

(event Custom|TryBuyDamage
  (if (>= (Variables|Default|GetCoins) (Variables|Default|GetCostMoreDamage))
    (CallFunction|SubstractCoins (Variables|Default|GetCostMoreDamage))
    (Variables|Default|SetFriendlyDamageAmount (+ 1e+01 (Variables|Default|GetFriendlyDamageAmount)))
    (Variables|Default|SetCostMoreDamage (+ (Variables|Default|GetCostMoreDamage) (/ (Variables|Default|GetCostMoreDamage) 5)))
    (bind _outactors (Actor|GetAllActorsOfClass "/Game/Blueprints/BP_FriendlyMinion.BP_FriendlyMinion_C"))
    (for _array_element _outactors
      (bind _asbp_friendly_minion (Utilities|Casting|CastToBP_FriendlyMinion _array_element))
      (Variables|/Game/Blueprints/BP_CharachterMinion.BP_CharachterMinion_C|SetDamageAmount _asbp_friendly_minion (Variables|Default|GetFriendlyDamageAmount)))))

(event Custom|TryBuyHealth
  (if (>= (Variables|Default|GetCoins) (Variables|Default|GetCostMoreHealth))
    (CallFunction|SubstractCoins (Variables|Default|GetCostMoreHealth))
    (Variables|Default|SetFriendlyMaxHealth (+ 1e+01 (Variables|Default|GetFriendlyMaxHealth)))
    (Variables|Default|SetCostMoreHealth (+ (Variables|Default|GetCostMoreHealth) (/ (Variables|Default|GetCostMoreHealth) 4)))
    (bind _outactors (Actor|GetAllActorsOfClass "/Game/Blueprints/BP_FriendlyMinion.BP_FriendlyMinion_C"))
    (for _array_element _outactors
      (bind _asbp_friendly_minion (Utilities|Casting|CastToBP_FriendlyMinion _array_element))
      (Variables|/Game/Blueprints/BPC_Health.BPC_Health_C|SetMaxHealth (Variables|/Game/Blueprints/BP_CharachterMinion.BP_CharachterMinion_C|GetBPC_Health _asbp_friendly_minion) (Variables|Default|GetFriendlyMaxHealth)))))

(event Custom|TryBuyHealingPower
  (if (>= (Variables|Default|GetCoins) (Variables|Default|GetCostMoreHealingPower))
    (CallFunction|SubstractCoins (Variables|Default|GetCostMoreHealingPower))
    (Variables|Default|SetCostMoreHealingPower (+ (Variables|Default|GetCostMoreHealingPower) (/ (Variables|Default|GetCostMoreHealingPower) 4)))
    (bind _outactors (Actor|GetAllActorsOfClass "/Game/Blueprints/BP_AbilityManager.BP_AbilityManager_C"))
    (Variables|/Game/Blueprints/BP_AbilityManager.BP_AbilityManager_C|SetHealAmount (Utilities|Array|Get(acopy) _outactors) (+ (Variables|/Game/Blueprints/BP_AbilityManager.BP_AbilityManager_C|GetHealAmount (Utilities|Array|Get(acopy) _outactors)) 5.0))))

(event Custom|MinionDied
  (params (IsFriendly :type Boolean))
  (bind _returnvalue (Game|GetCurrentLevelName true))
  (if (Utilities|Enum|Equal(Enum) _returnvalue "Tutorial0")
    (bind _outactors (Actor|GetAllActorsOfClass "/Game/Blueprints/BP_EnemyMinion.BP_EnemyMinion_C"))
    (if (== (Utilities|Array|Length _outactors) 0)
      (Game|OpenLevel(byName) "Sandbox"))
    (else
      (Variables|Default|SetEnemyDamageAmount (* (Variables|Default|GetEnemyDamageAmount) 1.05))
      (Variables|Default|SetEnemyMaxHealth (* (Variables|Default|GetEnemyMaxHealth) 1.05))
      (Variables|Default|SetMaxAmountOfActiveEnemies (+ (Variables|Default|GetMaxAmountOfActiveEnemies) (/ (Variables|Default|GetScore) 100))))))

(event Custom|IncreaseMaxEnemies
  (Math|Integer|IncrementInt (Variables|Default|GetMaxAmountOfActiveEnemies)))

(event EventBeginPlay
  (bind _returnvalue (Game|GetCurrentLevelName true))
  (if (Utilities|Enum|Equal(Enum) _returnvalue "Tutorial0")
    (Variables|Default|SetCoins 200)
    (Utilities|Time|SetTimerbyEvent (delegate Custom|IncreaseMaxEnemies) 4.0 true)))

(event EventTick
  (params (DeltaSeconds :type Float%20%28single-precision%29)))

(fn ConstructionScript)