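; Health component that tracks clamped health and a stackable shield, with damage, heal and death queries.
; DealDamage drains the shield first and passes overflow to health, then calls OnDead or OnDamage; full absorption calls neither.
; Heal works only while alive and calls OnHeal.
; AddShield sets ShieldTimer to its maximum, but Tick clears the shield while the timer is positive and decrements it only at or below zero.
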(event Custom|ResetHealth
  (Variables|Health|SetCurrentHealth (Variables|Health|GetMaxHealth)))

(event Custom|ResetShield
  (Variables|Shield|SetShieldAmount 0.0))

(event EventBeginPlay
  (CallFunction|ResetHealth)
  (CallFunction|ResetShield))

(event EventTick
  (params (DeltaSeconds :type Float%20%28single-precision%29))
  (if (<= (Variables|Shield|GetShieldTimer) 0.0)
    (Variables|Shield|SetShieldTimer (- (Variables|Shield|GetShieldTimer) DeltaSeconds))
    (else
      (CallFunction|ResetShield))))

(fn GetHealthPercentage
  (return (/ (Variables|Health|GetCurrentHealth) (Variables|Health|GetMaxHealth))))

(fn IsDead
  (return (== (CallFunction|GetHealthPercentage) 0.0)))

(fn DealDamage
  (params (Amount :type Float%20%28single-precision%29))
  (bind _isdead (CallFunction|IsDead))
  (bind _output_get (LocalVariables|SetDamageAmount Amount))
  (if (>= (Variables|Shield|GetShieldAmount) 0.0) ; TRUE = We have a shield
    (bind _output_get_2 (Variables|Shield|SetShieldAmount (- (Variables|Shield|GetShieldAmount) _output_get)))
    (if (< _output_get_2 0.0)
      (LocalVariables|SetDamageAmount (Math|Float|Absolute(Float) (Variables|Shield|GetShieldAmount))) ; Set damage equal to the amount\nof damage we overshot
      (CallFunction|ResetShield) ; Shield was in negative so put it on 0
      ;[1 1 1] Reduce HP
      ;;[1 1 1] Cache original health value
      (Variables|Default|SetoriginalHealth (Variables|Health|GetCurrentHealth) :!label _label)
      (bind _output_get_3 (Variables|Health|SetCurrentHealth (Math|Float|Clamp(Float) (- (Variables|Health|GetCurrentHealth) (LocalVariables|GetDamageAmount)) 0.0 (Variables|Health|GetMaxHealth))))
      ;;[1 1 1] Did this DoDamage cause the health to change and drop to 0?
      (if (and _isdead (> (Variables|Default|GetoriginalHealth) _output_get_3))
        (Default|CallOnDead)
        (else
          (Default|CallOnDamage)))
      (return _isdead))
    (else
      (goto _label))))

(fn Heal
  (params (Amount :type Float%20%28single-precision%29))
  (if (not (CallFunction|IsDead))
    (Variables|Health|SetCurrentHealth (Math|Float|Clamp(Float) (+ Amount (Variables|Health|GetCurrentHealth)) 0.0 (Variables|Health|GetMaxHealth)))
    (Default|CallOnHeal)))

(fn AddShield
  (params (Amount :type Float%20%28single-precision%29))
  (Variables|Shield|SetShieldAmount (+ Amount (Variables|Shield|GetShieldAmount)))
  (Variables|Shield|SetShieldTimer (Variables|Shield|GetShieldMaxTime)))