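; Minion character for both Friendly and Enemy sides, with tags selecting healthbar color plus health and damage from BP_MainGamemode.
; Attack hitbox overlaps with actors matching the AI controller's AttackTag start a looping damage timer, whose clear node is unwired.
; Tick retargets among overlapping minions; ClosestDistance never updates, so the last in range wins.
; BPC_Health events refresh the healthbar and, on death, notify the game mode, award coins for enemies and destroy the actor.
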(event OnDead(BPC_Health)
  (bind _tags (Variables|Actor|GetTags))
  (bind _returnvalue (Utilities|Array|ContainsItem _tags "Enemy"))
  (bind _asbp_main_gamemode (Utilities|Casting|CastToBP_MainGamemode (Game|GetGameMode))
    (:then
      (if _returnvalue
        (Default|AddCoins _asbp_main_gamemode (Variables|Default|GetCoinWorth)))
      (Default|MinionDied _asbp_main_gamemode (not _returnvalue)))
    (:CastFailed
      _))
  (Actor|DestroyActor))

(event OnComponentBeginOverlap(Attackhitbox)
  (params (OverlappedComponent :type Primitive%20Component%20Object%20Reference) (OtherActor :type Actor%20Object%20Reference) (OtherComp :type Primitive%20Component%20Object%20Reference) (OtherBodyIndex :type Integer) (bFromSweep :type Boolean) (SweepResult :type Hit%20Result%20Structure%20%28by%20ref%29))
  (bind _asbp_minion_ai (Utilities|Casting|CastToBP_MinionAI (Pawn|GetController)))
  (if (Utilities|Array|ContainsItem (Variables|/Script/Engine.Actor|GetTags OtherActor) (Variables|/Game/Blueprints/BP_MinionAI.BP_MinionAI_C|GetAttackTag _asbp_minion_ai))
    (Utilities|IsValid (Actor|GetComponentbyClass OtherActor "/Game/Blueprints/BPC_Health.BPC_Health_C")
      (:Is%20Valid
        (Variables|Default|SetCurrentDamageTarget OtherActor)
        (bind _returnvalue (Utilities|Time|SetTimerbyEvent (delegate Custom|DamageTarget) (Variables|Default|GetDamageDelay) true))
        (Variables|Default|SetDamageTimerHandle _returnvalue)))))

(event OnComponentEndOverlap(Attackhitbox)
  (params (OverlappedComponent :type Primitive%20Component%20Object%20Reference) (OtherActor :type Actor%20Object%20Reference) (OtherComp :type Primitive%20Component%20Object%20Reference) (OtherBodyIndex :type Integer))
  (if (== OtherActor (Variables|Default|GetCurrentDamageTarget))
    (Variables|Default|SetCurrentDamageTarget 0)))

(event OnDamage(BPC_Health)
  (bind _asbpw_healthbar (Utilities|Casting|CastToBPW_Healthbar (UserInterface|GetWidget (Variables|Default|GetHealthbar))))
  (Variables|/Game/Blueprints/HUD/BPW_Healthbar.BPW_Healthbar_C|SetCurrentHealthPercentage _asbpw_healthbar (Default|GetHealthPercentage (Variables|Default|GetBPC_Health))))

(event OnHeal(BPC_Health)
  (bind _asbpw_healthbar (Utilities|Casting|CastToBPW_Healthbar (UserInterface|GetWidget (Variables|Default|GetHealthbar))))
  (Variables|/Game/Blueprints/HUD/BPW_Healthbar.BPW_Healthbar_C|SetCurrentHealthPercentage _asbpw_healthbar (Default|GetHealthPercentage (Variables|Default|GetBPC_Health))))

(event Custom|SetMaxWalkingSpeed
  (params (MaxWalkSpeed :type Float%20%28single-precision%29))
  (Variables|/Script/Engine.CharacterMovementComponent|SetMaxWalkSpeed (Variables|Character|GetCharacterMovement) MaxWalkSpeed))

(event Custom|DamageTarget
  (bind _currentdamagetarget (Variables|Default|GetCurrentDamageTarget)
    (:then
      (bind _isdead (Default|DealDamage (Actor|GetComponentbyClass _currentdamagetarget "/Game/Blueprints/BPC_Health.BPC_Health_C") (Variables|Default|GetDamageAmount)))
      (if _isdead
        (CallFunction|UpdateTarget)))
    (:else)))

(event EventBeginPlay
  (bind _returnvalue (Game|GetGameMode))
  (bind _tags (Variables|Actor|GetTags))
  (bind _returnvalue_2 (Utilities|Array|ContainsItem _tags "Friendly"))
  (bind _asbp_main_gamemode (Utilities|Casting|CastToBP_MainGamemode _returnvalue))
  (bind _asbpw_healthbar (Utilities|Casting|CastToBPW_Healthbar (UserInterface|GetWidget (Variables|Default|GetHealthbar)))
    (:then
      (Variables|/Game/Blueprints/HUD/BPW_Healthbar.BPW_Healthbar_C|SetHealthColor _asbpw_healthbar (Math|Color|SelectColor "(R=0.979167,G=0.020399,B=0.040779,A=1.000000)" "(R=0.036250,G=0.966667,B=0.152849,A=1.000000)" (not _returnvalue_2))))
    (:CastFailed
      _))
  (Variables|Default|SetDamageAmount (Math|Float|SelectFloat (Variables|/Game/Blueprints/Main/BP_MainGamemode.BP_MainGamemode_C|GetFriendlyDamageAmount _asbp_main_gamemode) (Variables|/Game/Blueprints/Main/BP_MainGamemode.BP_MainGamemode_C|GetEnemyDamageAmount _asbp_main_gamemode) _returnvalue_2))
  (Variables|/Game/Blueprints/BPC_Health.BPC_Health_C|SetMaxHealth (Variables|Default|GetBPC_Health) (Math|Float|SelectFloat (Variables|/Game/Blueprints/Main/BP_MainGamemode.BP_MainGamemode_C|GetFriendlyMaxHealth _asbp_main_gamemode) (Variables|/Game/Blueprints/Main/BP_MainGamemode.BP_MainGamemode_C|GetEnemyMaxHealth _asbp_main_gamemode) _returnvalue_2)))

(event Collision|EventActorBeginOverlap
  (params (OtherActor :type Actor%20Object%20Reference)))

(event EventTick
  (params (DeltaSeconds :type Float%20%28single-precision%29))
  (CallFunction|UpdateTarget))

(fn ConstructionScript
  (bind _returnvalue (Rendering|Material|CreateDynamicMaterialInstance (Variables|Character|GetMesh) 0 0 "None" :!class /Script/Engine.PrimitiveComponent))
  (Rendering|Material|SetVectorParameterValue _returnvalue "BodyColor" (Variables|Default|GetBodyColor) :!class /Script/Engine.MaterialInstanceDynamic))

(fn UpdateTarget
  (LocalVariables|SetclosestDistance 9999.0)
  (for _array_element (Collision|GetOverlappingActors (Variables|Default|GetAttackhitbox) "BP_CharachterMinion_C" :!class /Script/Engine.PrimitiveComponent)
    (bind _asbp_minion_ai (Utilities|Casting|CastToBP_MinionAI (Pawn|GetController)))
    (if (Utilities|Array|ContainsItem (Variables|/Script/Engine.Actor|GetTags _array_element) (Variables|/Game/Blueprints/BP_MinionAI.BP_MinionAI_C|GetAttackTag _asbp_minion_ai))
      (if (< (Math|Vector|Distance(Vector) (Transformation|GetActorLocation _array_element) (Transformation|GetActorLocation)) (LocalVariables|GetclosestDistance))
        (Variables|Default|SetCurrentDamageTarget _array_element))))
  (return))