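; BP_Spawner periodically spawns AI pawns of a configurable class, up to a population limit.
; A looping timer runs SpawnLogic, which compares the world-wide count of that class with both its own threshold and the gamemode's active-enemy cap, with a fallback.
; Spawns use a random point in SpawnVolume or the actor's root.
; The AmountToSpawn loop returns after its first spawn.
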(event Custom|SpawnObjects
  (CallFunction|SpawnLogic))

(event EventBeginPlay
  (Utilities|Time|SetTimerbyEvent (delegate Custom|SpawnObjects) (Variables|Spawner|GetSpawnDelay) true))

(event Collision|EventActorBeginOverlap
  (params (OtherActor :type Actor%20Object%20Reference)))

(event EventTick
  (params (DeltaSeconds :type Float%20%28single-precision%29)))

(fn ConstructionScript)

(fn SpawnLogic
  (bind _returnvalue (Game|GetGameMode))
  (bind _spawnvolume (Variables|Default|GetSpawnVolume))
  (bind _defaultsceneroot (Variables|Default|GetDefaultSceneRoot))
  (bind (_asbp_main_gamemode _bsuccess) (Utilities|Casting|CastToBP_MainGamemode _returnvalue))
  (bind _outactors (Actor|GetAllActorsOfClass (Variables|Spawner|GetPawnToSpawn)))
  (if (and (< (Utilities|Array|Length _outactors) (Variables|Spawner|GetMaxThreshold)) (< (Utilities|Array|Length _outactors) (select _bsuccess (Variables|/Game/Blueprints/Main/BP_MainGamemode.BP_MainGamemode_C|GetMaxAmountOfActiveEnemies _asbp_main_gamemode) 10)))
    (for _index (range 0 (- (Variables|Spawner|GetAmountToSpawn) 1))
      (AI|SpawnAIFromClass (Variables|Spawner|GetPawnToSpawn) 0 (select (Variables|Spawner|GetUseSpawnVolume) (Math|Random|RandomPointinBoundingBox (Transformation|GetWorldLocation _spawnvolume) (Components|Box|GetScaledBoxExtent _spawnvolume)) (Transformation|GetWorldLocation _defaultsceneroot)) (Transformation|GetWorldRotation _defaultsceneroot) false 0)
      (return))))