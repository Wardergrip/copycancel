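; BP_CursorHologram is a cursor hologram actor whose cylinder mesh shows idle, healing or casting states.
; Separate events swap the VisualCylinder material, and ChangeLocation teleport-free moves the actor to a given location unless HoldPosition is set.
; ResetHologram clears the hold and restores the idle material.
; A function returns actors overlapping CylinderCollider, filtered by class, for callers to query what the hologram covers.
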(event Custom|SetIdleMat
  (Rendering|Material|SetMaterial (Variables|Default|GetVisualCylinder) 0 (Variables|Default|GetIdleMat)))

(event Custom|SetHealingMat
  (Rendering|Material|SetMaterial (Variables|Default|GetVisualCylinder) 0 (Variables|Default|GetHealMat)))

(event Custom|ChangeLocation
  (params (NewLocation :type Vector))
  (if (not (Variables|Default|GetHoldPosition))
    (Transformation|SetActorLocation NewLocation false false)))

(event Custom|ResetHologram
  (Variables|Default|SetHoldPosition false)
  (CallFunction|SetIdleMat))

(event Custom|SetCastingMat
  (Rendering|Material|SetMaterial (Variables|Default|GetVisualCylinder) 0 (Variables|Default|GetCastMat)))

(event EventBeginPlay)

(event Collision|EventActorBeginOverlap
  (params (OtherActor :type Actor%20Object%20Reference)))

(event EventTick
  (params (DeltaSeconds :type Float%20%28single-precision%29)))

(fn ConstructionScript)

(fn GetOverlappingActors
  (params (ClassFilter :type Actor%20Class%20Reference))
  (return (Collision|GetOverlappingActors (Variables|Default|GetCylinderCollider) ClassFilter :!class /Script/Engine.PrimitiveComponent)))