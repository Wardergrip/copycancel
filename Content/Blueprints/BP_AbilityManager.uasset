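; Ability manager actor that casts the selected area ability at a spawned cursor hologram, with cast time and cooldown.
; PrimaryFire locks the hologram and starts a cancellable timer, which fires the ability, starts the Tick-driven cooldown and schedules a hologram reset.
; Healing heals "Friendly"-tagged actors with BPC_Health overlapping the hologram and spawns particles on them.
; CycleUp and CycleDown are empty, though a GetNextAbility enum helper exists.
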(event Custom|PrimaryFire
  (bind _cursorhologram (Variables|Default|GetCursorHologram))
  ;[1 1 1] Try to cast ability
  (if (not (Variables|Default|GetIsOnCooldown))
    (Default|SetCastingMat _cursorhologram)
    (Variables|/Game/Blueprints/BP_CursorHologram.BP_CursorHologram_C|SetHoldPosition _cursorhologram true)
    (bind _returnvalue (Utilities|Time|SetTimerbyEvent (delegate Custom|FireCurrentAbility) (Variables|Default|GetCastTime)))
    (Variables|Default|SetAbilityTimerHandle _returnvalue)))

(event Custom|ChangeLocation
  (params (NewLocation :type Vector))
  ;[1 1 1] Change loc
  (Default|ChangeLocation (Variables|Default|GetCursorHologram) NewLocation))

(event Custom|FireAbility
  (params (Ability :type E_Abilities%20Enum :default "NewEnumerator0"))
  (bind _cursorhologram (Variables|Default|GetCursorHologram))
  (switch Utilities|FlowControl|Switch|SwitchonE_Abilities Ability
    (:NewEnumerator0
      ;[1 1 1] Heal ability
      ;;[1 1 1] Visual
      (Default|SetHealingMat _cursorhologram)
      (for _array_element (Default|GetOverlappingActors _cursorhologram)
        (Utilities|IsValid (Actor|GetComponentbyClass _array_element "/Game/Blueprints/BPC_Health.BPC_Health_C")
          (:Is%20Valid
            (if (Utilities|Array|ContainsItem (Variables|/Script/Engine.Actor|GetTags _array_element) "Friendly")
              (Default|Heal (Actor|GetComponentbyClass _array_element "/Game/Blueprints/BPC_Health.BPC_Health_C") (Variables|Default|GetHealAmount))
              (Effects|SpawnEmitteratLocation "/Game/Assets/PS_HealPE.PS_HealPE" (+ (Transformation|GetActorLocation _array_element) "0, 0, 0") "0, 0, 0" (* (Math|Vector|MakeVector 1.0 1.0 1.0) 1.0)))))))))

(event Custom|FireCurrentAbility
  ;[1 1 1] Try to cast ability
  (CallFunction|FireAbility (Variables|Default|GetCurrentAbility))
  (Utilities|Time|SetTimerbyEvent (delegate Custom|ResetHologram) (Variables|Default|GetAbilityEndHoverTime))
  (Variables|Default|SetCooldownTimer (Variables|Default|GetCooldown))
  (Variables|Default|SetIsOnCooldown true))

(event Custom|CancelAbilityCast
  ;[1 1 1] Player moved --> ability cancel
  (if (Variables|Default|GetAllowCancel)
    (Utilities|Time|ClearandInvalidateTimerbyHandle (Variables|Default|GetAbilityTimerHandle))
    (Default|ResetHologram (Variables|Default|GetCursorHologram))))

(event Custom|ResetHologram
  ;[1 1 1] Try to cast ability
  (Default|ResetHologram (Variables|Default|GetCursorHologram)))

(event Custom|CycleUp)

(event Custom|CycleDown)

(event EventBeginPlay
  (bind _returnvalue (Game|SpawnActorfromClass "/Game/Blueprints/BP_CursorHologram.BP_CursorHologram_C" (Math|Transform|MakeTransform "0, 0, 0" "0, 0, 0" "1,1,1") "Undefined" 0 0))
  (Variables|Default|SetCursorHologram _returnvalue))

(event Collision|EventActorBeginOverlap
  (params (OtherActor :type Actor%20Object%20Reference)))

(event EventTick
  (params (DeltaSeconds :type Float%20%28single-precision%29))
  (if (Variables|Default|GetIsOnCooldown)
    (bind _output_get (Variables|Default|SetCooldownTimer (- (Variables|Default|GetCooldownTimer) DeltaSeconds)))
    (if (<= _output_get 0.0)
      (Variables|Default|SetIsOnCooldown false))))

(fn ConstructionScript)

(fn GetPercentageCooldown
  (return (select (Variables|Default|GetIsOnCooldown) (/ (Variables|Default|GetCooldownTimer) (Variables|Default|GetCooldown)) 0.0)))

(fn GetNextAbility
  (params (CurrentAbility :type E_Abilities%20Enum :default "NewEnumerator0"))
  (bind _tempenum (LocalVariables|GetTempEnum))
  (bind _tempenum_2 (LocalVariables|GetTempEnum))
  (bind _returnvalue (Utilities|Array|FindItem _tempenum CurrentAbility))
  (bind _returnvalue_2 (+ _returnvalue 1))
  (Utilities|Array|Clear _tempenum)
  (bind _enumvalue (|ForEachE_Abilities)
    (:LoopBody
      (Utilities|Array|Add _tempenum _enumvalue))
    (:then
      (return (select (<= _returnvalue_2 (Utilities|Array|Length _tempenum)) (Utilities|Array|Get(acopy) _tempenum_2 _returnvalue_2) (Utilities|Array|Get(acopy) _tempenum_2))))))