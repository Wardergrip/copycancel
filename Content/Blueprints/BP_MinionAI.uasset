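; BP_MinionAI is the AI controller for minions, running BT_MinionBehavior on the controlled pawn.
; BeginPlay seeds the Blackboard with the player character, detection range and attack tag for the tree.
; Tick always draws a debug cylinder of the detection radius, colored by whether the attack tag is "Enemy".
; An older timer-driven system for finding tagged minions and moving to them remains, but its setup is disconnected.
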(event Custom|MoveToTarget
  ;[1 1 1] Old AI System
  (AI|AIMoveTo (Pawn|GetControlledPawn) "0, 0, 0" (Variables|Default|GetTargetToMoveTo) 5.0 false))

(event Custom|FindTarget
  ;[1 1 1] Old AI System
  (bind _outactors (Actor|GetAllActorsOfClasswithTag "/Game/Blueprints/BP_CharachterMinion.BP_CharachterMinion_C" (Variables|Default|GetAttackTag)))
  (bind _array_element (Utilities|Array|ForEachLoopwithBreak _outactors :!label _label)
    (:LoopBody
      (if (< (Math|Vector|Distance(Vector) (Transformation|GetActorLocation _array_element) (Transformation|GetActorLocation (Pawn|GetControlledPawn))) (Variables|Default|GetDetectionRange))
        (Utilities|FlowControl|Sequence
          (:then_0
            (Variables|Default|SetTargetToMoveTo _array_element))
          (:then_1
            (goto _label Break)))))
    (:Completed
      (Development|PrintString (Utilities|String|ToString(Integer) (Utilities|Array|Length _outactors))))))

(event EventBeginPlay
  (AI|RunBehaviorTree "/Game/AI/BT_MinionBehavior.BT_MinionBehavior")
  (bind _outactors (Actor|GetAllActorsOfClass "/Game/Blueprints/Main/BP_PlayerCharachter.BP_PlayerCharachter_C"))
  (AI|Components|Blackboard|SetValueasObject (Variables|Default|GetBlackboard) (Utilities|Name|MakeLiteralName "Player") (Utilities|Array|Get(acopy) _outactors))
  (AI|Components|Blackboard|SetValueasFloat (Variables|Default|GetBlackboard) (Utilities|Name|MakeLiteralName "DetectionRange") (Variables|Default|GetDetectionRange))
  (Class|BlackboardComponent|SetValueasString (Variables|Default|GetBlackboard) (Utilities|Name|MakeLiteralName "AttackTag") (Utilities|String|ToString(Name) (Variables|Default|GetAttackTag))))

(event EventTick
  (params (DeltaSeconds :type Float%20%28single-precision%29))
  (bind _returnvalue (Pawn|GetControlledPawn))
  (bind _returnvalue_2 (Transformation|GetActorLocation _returnvalue))
  (if true
    (Class|KismetSystemLibrary|DrawDebugCylinder _returnvalue_2 (+ _returnvalue_2 "0,0.000000,50.000000") (Variables|Default|GetDetectionRange) 12 (Math|Color|SelectColor "(R=0.000000,G=1.000000,B=0.082013,A=1.000000)" "(R=1.000000,G=0.000000,B=0.029716,A=1.000000)" (Utilities|Name|Equal(Name) (Variables|Default|GetAttackTag) "Enemy")) 0.0 0.0)))

(fn ConstructionScript)